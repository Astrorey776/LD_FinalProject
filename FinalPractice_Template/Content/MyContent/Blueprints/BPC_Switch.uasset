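; Lockable one-shot switch interactable that depresses its mesh when used and signals when the interaction completes.
; While locked, interacting only shows locked text; Unlock clears the lock, turns the material green and updates the prompt.
; Once unlocked, a DoOnce-gated Timeline lerps the mesh downward, then fires OnInteractionComplete and swaps the material.
; The construction script sets red or green material from IsLocked.
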(event EventStartEventsonInteract
  (if (Variables|Default|GetisLocked)
    (Rendering|Components|TextRender|SetText (Variables|Default|GetInteractUI) (Variables|Default|GetlockedText))
    (else
      (Utilities|FlowControl|DoOnce false
        (:Completed
          (bind _button (Timeline|Timeline Play)
            (:Update
              (Transformation|SetRelativeLocation (Variables|Default|GetStaticMesh) (Math|Vector|Lerp(Vector) "0, 0, 0" "0.000000,0.000000,-10.000000" _button) false false))
            (:Finished
              (Default|CallOnInteractionComplete)
              (Rendering|Material|SetMaterial (Variables|Default|GetStaticMesh) 0 "/Game/Materials/M_LDGrid_Local.M_LDGrid_Local"))))))))

(event EventUnlock
  (Variables|Default|SetisLocked false)
  (Rendering|Material|SetMaterial (Variables|Default|GetStaticMesh) 0 "/Game/Materials/M_LDGrid_Green.M_LDGrid_Green")
  (Rendering|Components|TextRender|SetText (Variables|Default|GetInteractUI) (Variables|Default|GetunlockedText)))

(fn ConstructionScript
  (bind _staticmesh (Variables|Default|GetStaticMesh))
  (|CallParentFunction)
  (if (Variables|Default|GetisLocked)
    (Rendering|Material|SetMaterial _staticmesh 0 "/Game/Materials/MI_LDGrid_Red.MI_LDGrid_Red")
    (else
      (Rendering|Material|SetMaterial _staticmesh 0 "/Game/Materials/M_LDGrid_Green.M_LDGrid_Green"))))