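; Barricade Blueprint made of four static meshes that collapses when interacted with.
; It overrides the parent's StartEventsonInteract event to enable physics on every piece, wake the bodies and signal interaction completion immediately.
; After a short delay the pieces are hidden in game, but they are not destroyed.
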(event EventStartEventsonInteract
  (bind _staticmesh3 (Variables|Default|GetStaticMesh3))
  (Physics|SetSimulatePhysics _staticmesh3 true)
  (Class|PrimitiveComponent|WakeAllRigidBodies _staticmesh3)
  (Default|CallOnInteractionComplete)
  (Utilities|FlowControl|Delay 2.0)
  (Development|SetHiddeninGame (Variables|Default|GetStaticMesh3) true false))

(fn ConstructionScript
  (|CallParentFunction))